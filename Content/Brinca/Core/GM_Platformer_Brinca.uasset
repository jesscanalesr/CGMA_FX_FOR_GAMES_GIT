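; Game mode for the Brinca platformer that tracks the player's coin count against a goal.
; SetCoins adds the given amount to the running total rather than replacing it, then prints the new total on screen.
; It then calls CheckGoal and prints a completion message whenever the total meets or exceeds CoinsGoal.
; GetCoins exposes the current total, and the event graph holds no active logic.
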(fn `CheckGoal`
  (returns (AchievedGoal :type Boolean))
  (if (>= (`self.CoinQty`) (`self.CoinsGoal`))
    (return true)
    (else
      (return false))))

(fn `GetCoins`
  (returns (Coins :type Integer))
  (return (`self.CoinQty`)))

(fn `SetCoins`
  (params (CoinsQty :type Integer))
  (bind _output_get (set `self.CoinQty` (+ (`self.CoinQty`) CoinsQty)))
  (`KismetSystemLibrary.PrintString` (`KismetStringLibrary.Conv_IntToString` _output_get) true true (struct :`R` 1.0 :`G` 0.800213 :`A` 1.0))
  (bind _achievedgoal (`self.CheckGoal`))
  (if _achievedgoal
    (`KismetSystemLibrary.PrintString` "You found all the coins!" true true (struct :`R` 1.0 :`G` 0.585886 :`A` 1.0) 10.0)))

(fn `UserConstructionScript`)