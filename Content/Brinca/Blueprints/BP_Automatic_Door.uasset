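; Automatic sliding door that opens when the player character enters its Box trigger and closes when they leave.
; Box overlap events filter for player 0's character, then play or reverse the OpenDoor timeline.
; The timeline's Transition track drives the Door's relative Y position, keeping X and Z unchanged.
; An OpenDoor-Forced event plays the same timeline to open the door without an overlap.
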(event `OpenDoor-Forced`
  (bind _door (`self.Door`))
  (bind (_relativelocation_x _relativelocation_y _relativelocation_z) (`KismetMathLibrary.BreakVector` (`SceneComponent.RelativeLocation` _door)))
  ;[0 0.09728 0.2] DoorOpenning
  (bind (_direction _transition) (`Timeline|OpenDoor` :!label _label)
    (:`Update`
      (`SceneComponent.K2_SetRelativeLocation` _door (`KismetMathLibrary.MakeVector` _relativelocation_x _transition _relativelocation_z) false false))))

(event `self.Box.OnComponentBeginOverlap`
  (params (OverlappedComponent :type "PrimitiveComponent Object Reference") (OtherActor :type "Actor Object Reference") (OtherComp :type "PrimitiveComponent Object Reference") (OtherBodyIndex :type Integer) (bFromSweep :type Boolean) (SweepResult :type "HitResult Structure (by ref)"))
  ;[0 0.09728 0.2] Check if the character overlapped
  (bind _isplayer (`self.CheckPlayerOverlap` OtherActor))
  (if _isplayer
    (goto _label)))

(event `self.Box.OnComponentEndOverlap`
  (params (OverlappedComponent :type "PrimitiveComponent Object Reference") (OtherActor :type "Actor Object Reference") (OtherComp :type "PrimitiveComponent Object Reference") (OtherBodyIndex :type Integer))
  ;[0 0.09728 0.2] Check if the character overlapped
  (bind _isplayer (`self.CheckPlayerOverlap` OtherActor))
  (if _isplayer
    (goto _label :!via `Reverse`)))

(fn `CheckPlayerOverlap`
  (params (Actor :type "Object Object Reference"))
  (returns (IsPlayer :type Boolean))
  ;[0 0.09728 0.2] Check if the character overlapped
  (if (== Actor (`GameplayStatics.GetPlayerCharacter` 0))
    (return true)
    (else
      (return false))))

(fn `UserConstructionScript`)