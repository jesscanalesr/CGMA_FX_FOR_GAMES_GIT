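; BP_Platform is a moving platform that changes color while the player character overlaps it.
; The construction script configures an InterpToMovement component with an editable Duration and two relative control points, from the platform mesh's location to BPosition.
; Box collision overlap events use CheckPlayerOverlap to filter for player 0's character, switching the mesh material to green on entry and blue on exit.
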(event `self.Box Collision.OnComponentBeginOverlap`
  (params (OverlappedComponent :type "PrimitiveComponent Object Reference") (OtherActor :type "Actor Object Reference") (OtherComp :type "PrimitiveComponent Object Reference") (OtherBodyIndex :type Integer) (bFromSweep :type Boolean) (SweepResult :type "HitResult Structure (by ref)"))
  ;[0 0.09728 0.2] Check Player Overlap
  (bind _isplayer (`self.CheckPlayerOverlap` OtherActor))
  (if _isplayer
    (`PrimitiveComponent.SetMaterial` (`self.Platform`) 0 "/AnimationSharing/AnimSharingGreen.AnimSharingGreen")))

(event `self.Box Collision.OnComponentEndOverlap`
  (params (OverlappedComponent :type "PrimitiveComponent Object Reference") (OtherActor :type "Actor Object Reference") (OtherComp :type "PrimitiveComponent Object Reference") (OtherBodyIndex :type Integer))
  ;[0 0.09728 0.2] Check Player Overlap
  (bind _isplayer (`self.CheckPlayerOverlap` OtherActor))
  (if _isplayer
    (`PrimitiveComponent.SetMaterial` (`self.Platform`) 0 "/AnimationSharing/AnimSharingBlue.AnimSharingBlue")))

(fn `CheckPlayerOverlap`
  (params (Actor :type "Object Object Reference"))
  (returns (IsPlayer :type Boolean))
  ;[0 0.09728 0.2] Check if the character overlapped
  (if (== Actor (`GameplayStatics.GetPlayerCharacter` 0))
    (return true)
    (else
      (return false))))

(fn `UserConstructionScript`
  (bind _interptomovement (`self.InterpToMovement`))
  (set `InterpToMovementComponent.Duration` (`self.Duration`) _interptomovement)
  (set `InterpToMovementComponent.ControlPoints` (`|MakeArray` (make `InterpControlPoint` (`SceneComponent.RelativeLocation` (`self.Platform`))) (make `InterpControlPoint` (`self.B Position`))) _interptomovement))